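; MyHUDR is the HUD for the respawn mechanic, owning the base layout widget and relaying timer updates to it.
; On PawnPossessed, CreateLayout creates W_BaseLayout for the owning player controller and adds it to the viewport, skipping creation if a valid one exists.
; UpdateTimerCount passes the timer value straight to that widget, while GetRespawnTime only returns zero.
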(event EventBeginPlay)

(event Collision|EventActorBeginOverlap
  (params (OtherActor :type Actor%20Object%20Reference)))

(event EventTick
  (params (DeltaSeconds :type Float%20%28single-precision%29)))

(event EventPawnPossessed
  (params (Pawn :type Pawn%20Object%20Reference))
  (CallFunction|CreateLayout))

(event EventUpdateTimerCount
  (params (Timer :type Float%20%28double-precision%29))
  (Default|UpdateTimerCount (Variables|Default|GetWCurrentLayout) Timer))

(fn ConstructionScript)

(fn CreateLayout
  (Variables|Default|GetWCurrentLayout
    (:then)
    (:else
      (bind _returnvalue (UserInterface|CreateWidget "/Game/Mechanics/Health/Widgets/W_BaseLayout.W_BaseLayout_C" (Game|Player|GetOwningPlayerController)))
      (bind _output_get (Variables|Default|SetWCurrentLayout _returnvalue))
      (UserInterface|Viewport|AddtoViewport _output_get 0))))

(fn GetRespawnTime
  (return 0.0))