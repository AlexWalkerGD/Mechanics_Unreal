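; Game mode that respawns a player on request at a randomly chosen PlayerStart.
; RequestRespawn calls SpawnNewPlayer, which destroys the controller's current pawn, spawns the default pawn class at GetRespawnPoint's transform and possesses it.
; GetRespawnPoint picks from all PlayerStart actors in the level.
; GetRespawnTime exposes NewTime but plays no part in this respawn flow, and a walk-speed assignment is left unconnected.
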(event EventBeginPlay)

(event EventTick
  (params (DeltaSeconds :type Float%20%28single-precision%29)))

(event EventRequestRespawn
  (params (PlayerController :type Player%20Controller%20Object%20Reference))
  (CallFunction|SpawnNewPlayer PlayerController))

(fn ConstructionScript)

(fn GetRespawnPoint
  (bind _outactors (Actor|GetAllActorsOfClass "/Script/Engine.PlayerStart"))
  (LocalVariables|SetPlayerStarts _outactors)
  (Utilities|IsValid (.OutItem (Utilities|Array|Random (LocalVariables|GetPlayerStarts)))
    (:Is%20Valid
      (return (Transformation|GetActorTransform (.OutItem (Utilities|Array|Random (LocalVariables|GetPlayerStarts))))))
    (:Is%20Not%20Valid
      (return ""))))

(fn SpawnNewPlayer
  (params (PlayerController :type Controller%20Object%20Reference))
  (bind _returnvalue (Pawn|GetControlledPawn PlayerController))
  (Utilities|IsValid PlayerController
    (:Is%20Valid
      (Utilities|IsValid _returnvalue
        (:Is%20Valid
          (Actor|DestroyActor _returnvalue))
        (:Is%20Not%20Valid
          _))
      (bind _returnvalue_2 (Game|SpawnActorfromClass (Variables|Default|GetDefaultPawnClass) (CallFunction|GetRespawnPoint) "Undefined" "MultiplyWithRoot" 0 0))
      (Pawn|Possess PlayerController _returnvalue_2))))

(fn GetRespawnTime
  (return (LocalVariables|GetNewTime)))