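; Base pickup item actor that lets an actor with an inventory component collect it by overlapping its sphere.
; On the server, overlap calls RequestCollectItem behind a DoOnce, then expires the actor shortly after success or re-arms after a delay on failure.
; RequestCollectItem returns false here as a stub.
; The skeletal mesh comes from ItemInfo, refreshed in the construction script and on its RepNotify.
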(event OnComponentBeginOverlap(Sphere)
  (params (OverlappedComponent :type Primitive%20Component%20Object%20Reference) (OtherActor :type Actor%20Object%20Reference) (OtherComp :type Primitive%20Component%20Object%20Reference) (OtherBodyIndex :type Integer) (bFromSweep :type Boolean) (SweepResult :type Hit%20Result%20Structure%20%28by%20ref%29))
  (bind _inventorycomponent (CallFunction|FindInventoryComponent OtherActor))
  (Networking|SwitchHasAuthority
    (:Authority
      (Utilities|IsValid _inventorycomponent
        (:Is%20Valid
          (Utilities|FlowControl|DoOnce false :!label _label
            (:Completed
              (bind _succedded (CallFunction|RequestCollectItem _inventorycomponent))
              (if _succedded
                (Actor|SetLifeSpan 0.1)
                (else
                  (Utilities|FlowControl|Delay 1.0)
                  (goto _label Reset))))))))))

(fn ConstructionScript
  (CallFunction|UpdateSkeletalMesh))

(fn RequestCollectItem
  (params (InventoryComponent :type AC%20Inventory%20Component%20Object%20Reference))
  (return false))

(fn OnRepItemInfo
  (CallFunction|UpdateSkeletalMesh))

(fn UpdateSkeletalMesh
  (Components|SkeletalMesh|SetSkeletalMeshAsset (Variables|Default|GetSkeletalMesh) (Variables|/Game/Mechanics/Inventory/Blueprints/Itens/Data/PrimaryDataAssets/PDA_ItemInfo.PDA_ItemInfo_C|GetSkMesh (Variables|Default|GetItemInfo))))