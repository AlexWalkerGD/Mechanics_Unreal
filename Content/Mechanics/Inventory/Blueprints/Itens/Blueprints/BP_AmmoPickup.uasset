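; BP_AmmoPickup is an inventory item pickup that holds an amount of ammo to collect.
; RequestCollectItem casts ItemInfo to PDA_AmmoInfo, lets the InventoryComponent try to collect the ammo, then keeps the returned remainder in AmmoAmount, allowing partial pickups.
; A RepNotify on AmmoAmount, along with BeginPlay, pushes the current count to the W3D_AmmoNumber widget on the pickup.
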(event EventBeginPlay
  (|CallParentFunction)
  (CallFunction|UpdateLocalWidget))

(fn ConstructionScript
  (|CallParentFunction))

(fn RequestCollectItem
  (params (InventoryComponent :type AC%20Inventory%20Component%20Object%20Reference))
  (bind _aspda_ammo_info (Utilities|Casting|CastToPDA_AmmoInfo (Variables|Default|GetItemInfo))
    (:then
      (bind (_succedded _ammoreimaining) (Default|TryCollectAmmo InventoryComponent _aspda_ammo_info (Variables|Default|GetAmmoAmount)))
      (Variables|Default|SetAmmoAmount _ammoreimaining)
      (return _succedded))
    (:CastFailed
      (return false))))

(fn OnRepAmmoAmount
  (CallFunction|UpdateLocalWidget))

(fn UpdateLocalWidget
  (bind _asw3d_ammo_number (Utilities|Casting|CastToW3D_AmmoNumber (UserInterface|GetWidget (Variables|Default|GetWidget))))
  (Default|UpdateAmmo _asw3d_ammo_number (Variables|Default|GetAmmoAmount)))