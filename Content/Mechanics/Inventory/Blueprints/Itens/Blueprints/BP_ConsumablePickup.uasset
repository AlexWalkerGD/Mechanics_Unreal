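; BP_ConsumablePickup is an inventory pickup that holds a replicated amount of a consumable item.
; On a collect request it casts its item info to PDA_ConsumableInfo, passes it to the inventory component's TryCollectConsumable, and keeps the remainder, allowing partial collection.
; BeginPlay and the amount's OnRep call UpdateLocalWidget, which is currently empty because its W3D_AmmoNumber update logic is disconnected.
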(event EventBeginPlay
  (|CallParentFunction)
  (CallFunction|UpdateLocalWidget))

(fn ConstructionScript
  (|CallParentFunction))

(fn RequestCollectItem
  (params (InventoryComponent :type AC%20Inventory%20Component%20Object%20Reference))
  (bind _aspda_consumable_info (Utilities|Casting|CastToPDA_ConsumableInfo (Variables|Default|GetItemInfo))
    (:then
      (bind (_succedded _consumablereimaining) (Default|TryCollectConsumable InventoryComponent _aspda_consumable_info (Variables|Default|GetConsumableAmount)))
      (Variables|Default|SetConsumableAmount _consumablereimaining)
      (return _succedded))
    (:CastFailed
      (return false))))

(fn OnRepConsumableAmount
  (CallFunction|UpdateLocalWidget))

(fn UpdateLocalWidget)