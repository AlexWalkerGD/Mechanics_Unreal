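; Actor component that tracks an actor's health and death state for damage handling.
; ApplyDamage subtracts from Health while the owner is alive and sets IsDead once Health reaches zero or below.
; Replicated Health and IsDead use OnRep functions to broadcast health-change and death events.
; Getters expose raw health, normalized health against MaxHealth, and the dead state.
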(event EventBeginPlay)

(event EventTick
  (params (DeltaSeconds :type Float%20%28single-precision%29)))

(fn OnRepMaxHealth)

(fn OnRepHealth
  (Default|CallOnHealthChange self))

(fn OnRepIsDead
  (Default|CallOnDied))

(fn GetHealth
  (return (Variables|Default|GetHealth)))

(fn GetDeadState
  (return (Variables|Default|GetIsDead)))

(fn GetNormalizadHealth
  (return (/ (Variables|Default|GetHealth) (Variables|Default|GetMax%20Health))))

(fn ApplyDamage
  (params (Damage :type Float%20%28double-precision%29))
  (if (CallFunction|CanReceiveDamage)
    (bind _output_get (Variables|Default|SetHealth (- (Variables|Default|GetHealth) Damage)))
    (if (<= _output_get 0.0)
      (Variables|Default|SetIsDead true))))

(fn CanReceiveDamage
  (return (not (Variables|Default|GetIsDead))))