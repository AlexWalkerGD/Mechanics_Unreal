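; BP_WeaponPickup is a weapon pickup that hands a weapon and its clip ammo to the collecting inventory component.
; RequestCollectItem calls TryCollectWeapon; on a swap, the pickup takes on the returned weapon and ammo and returns false, otherwise it returns true.
; A widget displays the clip ammo, refreshed on BeginPlay and through the RepNotify on ClipAmmoAmount.
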(event EventBeginPlay
  (|CallParentFunction)
  (CallFunction|UpdateLocalWidget))

(fn ConstructionScript
  (|CallParentFunction))

(fn RequestCollectItem
  (params (InventoryComponent :type AC%20Inventory%20Component%20Object%20Reference))
  (bind _aspda_weapon_info (Utilities|Casting|CastToPDA_WeaponInfo (Variables|Default|GetItemInfo))
    (:then
      (bind (_swapweapon _weapontoswap _clipammotoswap) (Default|TryCollectWeapon InventoryComponent _aspda_weapon_info (Variables|Default|GetClipAmmoAmount)))
      (if _swapweapon
        (Variables|Default|SetItemInfo _weapontoswap)
        (Variables|Default|SetClipAmmoAmount _clipammotoswap)
        (return false)
        (else
          (return true))))
    (:CastFailed
      (return false))))

(fn OnRepClipAmmoAmount
  (CallFunction|UpdateLocalWidget))

(fn UpdateLocalWidget
  (bind _asw3d_ammo_number (Utilities|Casting|CastToW3D_AmmoNumber (UserInterface|GetWidget (Variables|Default|GetWidget))))
  (Default|UpdateAmmo _asw3d_ammo_number (Variables|Default|GetClipAmmoAmount)))