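; HUD for the weapon mechanics that creates the on-screen layout and inventory widgets and controls when the inventory is shown.
; On BeginPlay it adds both widgets to the viewport and keeps the inventory hidden.
; Visibility reveals the inventory with the mouse cursor and Game and UI input focused on it.
; Hidden clears the inventory list, hides the widget and cursor, and restores game-only input.
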(event EventBeginPlay
  (bind _returnvalue (Game|Player|GetOwningPlayerController))
  (bind _returnvalue_2 (UserInterface|CreateWidget "/Game/Mechanics/Weapon/Widgets/W_Layout.W_Layout_C" _returnvalue))
  (UserInterface|Viewport|AddtoViewport _returnvalue_2 0)
  (bind _returnvalue_3 (UserInterface|CreateWidget "/Game/Mechanics/Inventory/Widget/W_Inventory.W_Inventory_C" _returnvalue))
  (bind _output_get (Variables|Default|SetWInventory _returnvalue_3))
  (UserInterface|Viewport|AddtoViewport _returnvalue_3 0)
  (Widget|SetVisibility _output_get "Hidden"))

(fn ConstructionScript)

(fn Visibility
  (bind _returnvalue (Game|GetPlayerController 0))
  (bind _winventory (Variables|Default|GetWInventory))
  (Widget|SetVisibility _winventory "Visible")
  (Input|SetInputModeGameandUI _returnvalue _winventory "DoNotLock" true false)
  (Variables|/Script/Engine.PlayerController|SetbShowMouseCursor _returnvalue true))

(fn Hidden
  (bind _returnvalue (Game|GetPlayerController 0))
  (bind _winventory (Variables|Default|GetWInventory))
  (Widget|Panel|ClearChildren (Variables|/Game/Mechanics/Inventory/Widget/W_Inventory.W_Inventory_C|GetList _winventory))
  (Widget|SetVisibility _winventory "Hidden")
  (Input|SetInputModeGameOnly _returnvalue false)
  (Variables|/Script/Engine.PlayerController|SetbShowMouseCursor _returnvalue false))